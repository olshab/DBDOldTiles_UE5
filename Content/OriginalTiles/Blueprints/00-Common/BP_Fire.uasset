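; BP_Fire is a fire effect actor that endlessly alternates between full flames and a smoky state.
; From BeginPlay, a looping chain of randomized delays toggles named emitters on the PFire particle system through FireNormal and FireSmoke, briefly overlapping both groups when shifting to smoke.
; A Spawn helper sets per-emitter float parameters on a particle component but is not called in these graphs.
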(event EventBeginPlay
  (CallFunction|FireSmoke (Variables|Default|GetP_Fire) false)
  (CallFunction|FireNormal (Variables|Default|GetP_Fire) true)
  (Utilities|FlowControl|Delay (Math|Random|RandomFloatinRange 1e+01 2e+01) :!label _label)
  (CallFunction|FireNormal (Variables|Default|GetP_Fire) true)
  (CallFunction|FireSmoke (Variables|Default|GetP_Fire) true)
  (Utilities|FlowControl|Delay 1.0)
  (CallFunction|FireNormal (Variables|Default|GetP_Fire) false)
  (CallFunction|FireSmoke (Variables|Default|GetP_Fire) true)
  (Utilities|FlowControl|Delay (Math|Random|RandomFloatinRange 7.0 15.0))
  (CallFunction|FireSmoke (Variables|Default|GetP_Fire) true)
  (CallFunction|FireNormal (Variables|Default|GetP_Fire) true)
  (CallFunction|FireSmoke (Variables|Default|GetP_Fire) false)
  (CallFunction|FireNormal (Variables|Default|GetP_Fire) true)
  (goto _label))

(fn ConstructionScript)

(fn FireSmoke
  (params (FX :type Particle%20System%20Component%20Object%20Reference) (smoke :type Boolean))
  (Effects|Components|ParticleSystem|SetEmitterEnable FX "S_Smoke2" smoke)
  (Effects|Components|ParticleSystem|SetEmitterEnable FX "S_SmokeGround" smoke)
  (Effects|Components|ParticleSystem|SetEmitterEnable FX "S_Fire0" smoke))

(fn FireNormal
  (params (FX :type Particle%20System%20Component%20Object%20Reference) (Normal :type Boolean))
  (Effects|Components|ParticleSystem|SetEmitterEnable FX "Smoke1" Normal)
  (Effects|Components|ParticleSystem|SetEmitterEnable FX "Smoke2" Normal)
  (Effects|Components|ParticleSystem|SetEmitterEnable FX "Fire0" Normal)
  (Effects|Components|ParticleSystem|SetEmitterEnable FX "Flames1" Normal)
  (Effects|Components|ParticleSystem|SetEmitterEnable FX "Flames2" Normal)
  (Effects|Components|ParticleSystem|SetEmitterEnable FX "Flames3" Normal))

(fn Spawn
  (params (Spawn :type Particle%20System%20Component%20Object%20Reference) (Smoke1 :type Float%20%28double-precision%29) (Smoke2 :type Float%20%28double-precision%29) (F_Smoke2 :type Float%20%28double-precision%29) (Fire0 :type Float%20%28double-precision%29) (F_Fire0 :type Float%20%28double-precision%29) (Flames1 :type Float%20%28double-precision%29) (Flames2 :type Float%20%28double-precision%29) (Flames3 :type Float%20%28double-precision%29) (F_Flames1 :type Float%20%28double-precision%29) (F_Flames2 :type Float%20%28double-precision%29) (F_Flames3 :type Float%20%28double-precision%29))
  (Effects|Components|ParticleSystem|SetFloatParameter Spawn "Smoke1" Smoke1)
  (Effects|Components|ParticleSystem|SetFloatParameter Spawn "Smoke2" Smoke2)
  (Effects|Components|ParticleSystem|SetFloatParameter Spawn "F_Smoke2" F_Smoke2)
  (Effects|Components|ParticleSystem|SetFloatParameter Spawn "Fire0" Fire0)
  (Effects|Components|ParticleSystem|SetFloatParameter Spawn "F_Fire0" F_Fire0)
  (Effects|Components|ParticleSystem|SetFloatParameter Spawn "Flames1" Flames1)
  (Effects|Components|ParticleSystem|SetFloatParameter Spawn "Flames2" Flames2)
  (Effects|Components|ParticleSystem|SetFloatParameter Spawn "Flames3" Flames3)
  (Effects|Components|ParticleSystem|SetFloatParameter Spawn "F_Flames1" F_Flames1)
  (Effects|Components|ParticleSystem|SetFloatParameter Spawn "F_Flames2" F_Flames2)
  (Effects|Components|ParticleSystem|SetFloatParameter Spawn "F_Flames3" F_Flames3))