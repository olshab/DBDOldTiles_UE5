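; Horologium mod actor for Dead by Daylight that visually replaces level actors using a data table chosen by the map's theme.
; Table row names are class paths, with content file paths converted to /Game/ class paths and loaded synchronously.
; Each tick until the level is ready, it hides matching actors' components, recursing into child actors and sparing listed names.
; Once ready, it spawns each row's replacement at those actors' transforms and stops processing.
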(event Custom|ProcessDataTable
  (bind _outrownames (DataTable|GetDataTableRowNames (Variables|Default|GetActorOverrideDataTable)))
  (for _array_element _outrownames
    (bind _output_get (Variables|Default|SetRowName _array_element))
    (bind _returnvalue (Utilities|GetDataTableRow (Variables|Default|GetActorOverrideDataTable) _output_get)
      (:then
        (Variables|Default|SetCurrentRow _returnvalue)
        (bind _returnvalue_2 (Utilities|LoadClassAssetBlocking (Class|KismetSystemLibrary|ToSoftClassRef(SoftClassPath) (Class|KismetSystemLibrary|MakeSoftClassPath (CallFunction|GetPackageName (Utilities|String|ToString(Name) (Variables|Default|GetRowName)))))))
        (bind _asactor (Utilities|Casting|CastToActorClass _returnvalue_2))
        (bind _outactors (Actor|GetAllActorsOfClass _asactor))
        (bind _output_get_2 (Variables|Default|SetTopLevelActors _outactors))
        (for _array_element_2 _output_get_2
          (CallFunction|HideAllComponents _array_element_2 (Utilities|Struct|BreakActorClassOverride (Variables|Default|GetCurrentRow))))))))

(event Custom|SpawnReplacedBlueprints
  (bind _outrownames (DataTable|GetDataTableRowNames (Variables|Default|GetActorOverrideDataTable)))
  (for _array_element _outrownames
    (bind _output_get (Variables|Default|SetRowName _array_element))
    (bind _returnvalue (Utilities|GetDataTableRow (Variables|Default|GetActorOverrideDataTable) _output_get)
      (:then
        (Variables|Default|SetCurrentRow _returnvalue)
        (bind _returnvalue_2 (Utilities|LoadClassAssetBlocking (Class|KismetSystemLibrary|ToSoftClassRef(SoftClassPath) (Class|KismetSystemLibrary|MakeSoftClassPath (CallFunction|GetPackageName (Utilities|String|ToString(Name) (Variables|Default|GetRowName)))))))
        (bind _asactor (Utilities|Casting|CastToActorClass _returnvalue_2))
        (bind _outactors (Actor|GetAllActorsOfClass _asactor))
        (bind _output_get_2 (Variables|Default|SetTopLevelActors _outactors))
        (for _array_element_2 _output_get_2
          (bind _returnvalue_3 (Utilities|LoadClassAssetBlocking (Utilities|Struct|BreakActorClassOverride (Variables|Default|GetCurrentRow))))
          (bind _asactor_2 (Utilities|Casting|CastToActorClass _returnvalue_3))
          (Game|SpawnActorfromClass _asactor_2 (Transformation|GetActorTransform _array_element_2) "AlwaysSpawn" "MultiplyWithRoot" 0 0))))))

(event EventTick
  (params (DeltaSeconds :type Float%20%28single-precision%29))
  (Utilities|FlowControl|Sequence
    (:then_0
      (if (Variables|Default|GetShouldProcessActors)
        (bind _datatable (CallFunction|GetActorOverrideDataTable))
        (Variables|Default|SetActorOverrideDataTable _datatable)
        (CallFunction|ProcessDataTable)))
    (:then_1
      (if (and (Variables|Default|GetShouldProcessActors) (Class|DBDGameState|IsLevelReadytoPlay (.AsDBDGame%20State (Utilities|Casting|CastToDBDGameState (Game|GetGameState)))))
        (Variables|Default|SetShouldProcessActors false)
        (CallFunction|SpawnReplacedBlueprints)))))

(fn ConstructionScript)

(fn GetPackageName
  (params (String :type String))
  (if (Utilities|String|StartsWith String "/" "CaseSensitive")
    (return String)
    (else
      (return (Utilities|String|Append (Utilities|String|Append (Utilities|String|Append (Utilities|String|Replace (.LeftS (Utilities|String|Split String "." "CaseSensitive" "FromEnd")) "DeadByDaylight/Content/" "/Game/" "CaseSensitive") ".") (.LeftS (Utilities|String|Split (.RightS (Utilities|String|Split String "/" "CaseSensitive" "FromEnd")) "." "CaseSensitive"))) "_C")))))

(fn HideAllComponents
  (params (CurrentActor :type Actor%20Object%20Reference) (IgnoreComponents :type Array%20of%20Strings))
  (Utilities|FlowControl|Sequence
    (:then_0
      (bind _output_get (LocalVariables|SetSceneComponents (Actor|GetComponentsByClass CurrentActor "/Script/Engine.SceneComponent")))
      (for _array_element _output_get
        (bind _output_get_2 (LocalVariables|SetCurrentComponent _array_element))
        (if (not (Utilities|Array|ContainsItem IgnoreComponents (Utilities|GetObjectName _output_get_2)))
          (Rendering|SetVisibility (LocalVariables|GetCurrentComponent) false false)
          (Development|SetHiddeninGame (LocalVariables|GetCurrentComponent) true false))))
    (:then_1
      (bind _output_get_3 (LocalVariables|SetChildActorComponents (Actor|GetComponentsByClass CurrentActor "/Script/Engine.ChildActorComponent")))
      (for _array_element_2 _output_get_3
        (CallFunction|HideAllComponents (Variables|/Script/Engine.ChildActorComponent|GetChildActor _array_element_2) (Utilities|Array|MakeArray ""))))))

(fn GetThemeName
  (return (Variables|/Script/DeadByDaylight.MapData|GetThemeName (Variables|/Script/DeadByDaylight.ProceduralLevelBuilder|Get_mapData (Class|DBDUtilities|GetBuilder self)))))

(fn GetActorOverrideDataTable
  (bind _returnvalue (Utilities|LoadAssetBlocking (.Value (Utilities|Map|Find (Variables|Default|GetThemeToDataTable) (CallFunction|GetThemeName)))))
  (bind _asdata_table (Utilities|Casting|CastToDataTable _returnvalue))
  (return _asdata_table))